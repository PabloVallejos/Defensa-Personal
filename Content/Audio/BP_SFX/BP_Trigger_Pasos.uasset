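; BP_Trigger_Pasos is a trigger volume that plays the Pasos footstep sound as 2D audio while the player moves inside it.
; Box overlap events set InRoom, with only the begin event checking for the player character.
; Tick updates IsMooving from the player's velocity and calls PlaySound2D every frame both flags are true, with no interval between plays.
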(event OnComponentBeginOverlap(Box)
  (params (OverlappedComponent :type Primitive%20Component%20Object%20Reference) (OtherActor :type Actor%20Object%20Reference) (OtherComp :type Primitive%20Component%20Object%20Reference) (OtherBodyIndex :type Integer) (bFromSweep :type Boolean) (SweepResult :type Hit%20Result%20Structure%20%28by%20ref%29))
  (if (== OtherActor (Game|GetPlayerCharacter 0))
    (Variables|Default|SetInRoom true)))

(event OnComponentEndOverlap(Box)
  (params (OverlappedComponent :type Primitive%20Component%20Object%20Reference) (OtherActor :type Actor%20Object%20Reference) (OtherComp :type Primitive%20Component%20Object%20Reference) (OtherBodyIndex :type Integer))
  (Variables|Default|SetInRoom false))

(event EventTick
  (params (DeltaSeconds :type Float%20%28single-precision%29))
  (Utilities|FlowControl|Sequence
    (:then_0
      (if (Variables|Default|GetIsMooving)
        (if (Variables|Default|GetInRoom)
          (Audio|PlaySound2D (Variables|Default|GetPasos) 1.0 1.0 0.0 0 0))))
    (:then_1
      (Variables|Default|SetIsMooving (> (Math|Vector|VectorLength (Transformation|GetVelocity (Game|GetPlayerCharacter 0))) 0.0)))))

(fn ConstructionScript)
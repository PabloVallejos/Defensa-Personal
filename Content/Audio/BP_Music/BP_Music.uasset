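; BP_Music is a layered music actor that adds a second music layer when its trigger is overlapped.
; On BeginPlay it sets the base sound mix, plays layer one as 2D sound, and starts layers two and three muted through sound class overrides.
; The first TriggerMusic overlap, by any actor, re-applies the layer two override with default values to bring it in.
; Layer three stays muted in this graph.
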(event OnComponentBeginOverlap(TriggerMusic)
  (params (OverlappedComponent :type Primitive%20Component%20Object%20Reference) (OtherActor :type Actor%20Object%20Reference) (OtherComp :type Primitive%20Component%20Object%20Reference) (OtherBodyIndex :type Integer) (bFromSweep :type Boolean) (SweepResult :type Hit%20Result%20Structure%20%28by%20ref%29))
  (Utilities|FlowControl|DoOnce false
    (:Completed
      (Audio|SetSoundMixClassOverride "/Game/Audio/My_Mix.My_Mix" "/Game/Audio/Music_Layer2.Music_Layer2" 1.0 1.0 1.0 true))))

(event EventBeginPlay
  (Class|GameplayStatics|SetBaseSoundMix "/Game/Audio/My_Mix.My_Mix")
  (Utilities|FlowControl|Sequence
    (:then_0
      (Audio|PlaySound2D "/Game/Audio/Music/Def_Music_Layer_1.Def_Music_Layer_1" 1.0 1.0 0.0 0 0 false))
    (:then_1
      (Audio|SetSoundMixClassOverride "/Game/Audio/My_Mix.My_Mix" "/Game/Audio/Music_Layer2.Music_Layer2" 0.0 1.0 0.0 true)
      (Audio|Components|Audio|Play (Variables|Default|GetLayer2) 0.0))
    (:then_2
      (Audio|SetSoundMixClassOverride "/Game/Audio/My_Mix.My_Mix" "/Game/Audio/Music_Layer3.Music_Layer3" 0.0 1.0 0.0 true)
      (Audio|Components|Audio|Play (Variables|Default|GetLayer3) 0.0))))

(fn ConstructionScript)
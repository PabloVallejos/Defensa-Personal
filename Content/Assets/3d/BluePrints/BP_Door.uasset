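; BP_Door is a door that swings open automatically when the first-person character enters its box trigger and closes when the character leaves.
; A timeline drives the SMDoor mesh yaw up to 90 degrees times its DoorTime track, playing on overlap begin and reversing on overlap end.
; Opening plays a 2D sound at once, while the closing sound waits on a delay set by the current DoorTime value.
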(event OnComponentBeginOverlap(Box)
  (params (OverlappedComponent :type Primitive%20Component%20Object%20Reference) (OtherActor :type Actor%20Object%20Reference) (OtherComp :type Primitive%20Component%20Object%20Reference) (OtherBodyIndex :type Integer) (bFromSweep :type Boolean) (SweepResult :type Hit%20Result%20Structure%20%28by%20ref%29))
  (Utilities|Casting|CastToBP_FirstPersonCharacter OtherActor)
  (Utilities|FlowControl|Sequence
    (:then_0
      (bind _doortime (Timeline|Timeline Play)
        (:Update
          (Transformation|SetRelativeRotation (Variables|Default|GetSM_Door) (Math|Rotator|MakeRotator 0.0 0.0 (* _doortime 9e+01)) false false))))
    (:then_1
      (Audio|PlaySound2D "/Game/Audio/SFX/SC_Door.SC_Door" 1.0 1.0 0.0 0 0))))

(event OnComponentEndOverlap(Box)
  (params (OverlappedComponent :type Primitive%20Component%20Object%20Reference) (OtherActor :type Actor%20Object%20Reference) (OtherComp :type Primitive%20Component%20Object%20Reference) (OtherBodyIndex :type Integer))
  ;[1 1 1] Cierra La Puerta
  (Utilities|Casting|CastToBP_FirstPersonCharacter OtherActor)
  (Utilities|FlowControl|Sequence
    (:then_0
      (bind _doortime (Timeline|Timeline Reverse)
        (:Update
          (Transformation|SetRelativeRotation (Variables|Default|GetSM_Door) (Math|Rotator|MakeRotator 0.0 0.0 (* _doortime 9e+01)) false false))))
    (:then_1
      (Utilities|FlowControl|Delay _doortime)
      (Audio|PlaySound2D "/Game/Audio/SFX/SC_Close.SC_Close" 1.0 1.0 0.0 0 0))))

(fn ConstructionScript)
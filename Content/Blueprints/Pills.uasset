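; Sanity pill pickup that starts with its mesh hidden at BeginPlay.
; The checkPillRespawn event reveals the mesh and sets the TrueFalse flag that gates pickup.
; When that flag is set, a first-person character overlapping the capsule gains Heal on San, its UI updates, and the pill destroys itself.
; Nodes that would write a Pills array to BP_GameState are left unconnected and never run.
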(event OnComponentBeginOverlap(Capsule)
  (params (OverlappedComponent :type Primitive%20Component%20Object%20Reference) (OtherActor :type Actor%20Object%20Reference) (OtherComp :type Primitive%20Component%20Object%20Reference) (OtherBodyIndex :type Integer) (bFromSweep :type Boolean) (SweepResult :type Hit%20Result%20Structure%20%28by%20ref%29))
  ;[1 1 1] Player Drink the Pill and destroy
  (if (Variables|Default|GettrueFalse)
    (bind _asbp_first_person_character (Utilities|Casting|CastToBP_FirstPersonCharacter OtherActor))
    (bind _output_get (Variables|/Game/FirstPerson/Blueprints/BP_FirstPersonCharacter.BP_FirstPersonCharacter_C|SetSan _asbp_first_person_character (+ (Variables|/Game/FirstPerson/Blueprints/BP_FirstPersonCharacter.BP_FirstPersonCharacter_C|GetSan _asbp_first_person_character) (Variables|Default|GetHeal))))
    (Default|UpdateSanity (Variables|/Game/FirstPerson/Blueprints/BP_FirstPersonCharacter.BP_FirstPersonCharacter_C|GetUI _asbp_first_person_character) _output_get)
    (Actor|DestroyActor)))

(event Custom|checkPillRespawn
  ;[1 1 1] Check pill Respawn
  (Rendering|ToggleVisibility (Variables|Default|GetStaticMesh) true)
  (Variables|Default|SettrueFalse true))

(event EventBeginPlay
  ;[1 1 1] Initialize GameSate
  (Rendering|ToggleVisibility (Variables|Default|GetStaticMesh) false))

(fn ConstructionScript)
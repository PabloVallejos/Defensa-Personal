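; Game state Blueprint that tracks every Target and Pills actor and decides how the session ends.
; BeginPlay caches both sets and calls WinCondition.
; If Sleepy stays set through a 60-second delay, the player loses control with a Spanish going-to-sleep message; if initially unset, a HitCounter matching the target count shows a win and also disables control.
; MAKEALLSPOOKY switches every Target to its spooky look.
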(event Custom|Win%20Condition
  (params (DeltaSeconds :type Float%20%28single-precision%29))
  (if (Variables|Default|GetSleepy)
    ;[1 1 1] Si no sale del cuarto
    (Utilities|FlowControl|Delay 6e+01)
    (if (Variables|Default|GetSleepy)
      (bind _returnvalue (Actor|GetActorOfClass "/Game/FirstPerson/Blueprints/BP_FirstPersonCharacter.BP_FirstPersonCharacter_C"))
      (Variables|/Game/FirstPerson/Blueprints/BP_FirstPersonCharacter.BP_FirstPersonCharacter_C|SetDamaged _returnvalue false)
      (Variables|/Game/FirstPerson/Blueprints/BP_FirstPersonCharacter.BP_FirstPersonCharacter_C|SetControllable _returnvalue false)
      (Variables|/Script/UMG.TextBlock|SetText (Variables|/Game/Blueprints/Level_UI.Level_UI_C|GetGOT (Variables|/Game/FirstPerson/Blueprints/BP_FirstPersonCharacter.BP_FirstPersonCharacter_C|GetUI _returnvalue)) "Alv, me voy a mimir -_-"))
    (else
      ;[1 1 1] Si sale del cuarto
      (bind _returnvalue_2 (Actor|GetActorOfClass "/Game/FirstPerson/Blueprints/BP_FirstPersonCharacter.BP_FirstPersonCharacter_C"))
      (if (== (Variables|/Game/FirstPerson/Blueprints/BP_FirstPersonCharacter.BP_FirstPersonCharacter_C|GetHit%20Counter _returnvalue_2) (Utilities|Array|Length (Variables|Default|GetTargets)))
        (Variables|/Script/UMG.TextBlock|SetText (Variables|/Game/Blueprints/Level_UI.Level_UI_C|GetGOT (Variables|/Game/FirstPerson/Blueprints/BP_FirstPersonCharacter.BP_FirstPersonCharacter_C|GetUI _returnvalue_2)) "¡GANASTE!")
        (Variables|/Game/FirstPerson/Blueprints/BP_FirstPersonCharacter.BP_FirstPersonCharacter_C|SetDamaged _returnvalue_2 false)
        (Variables|/Game/FirstPerson/Blueprints/BP_FirstPersonCharacter.BP_FirstPersonCharacter_C|SetControllable _returnvalue_2 false)))))

(event EventBeginPlay
  ;[1 1 1] Agarra todos los "Target"
  (bind _outactors (Actor|GetAllActorsOfClass "/Game/Blueprints/Target.Target_C"))
  (Variables|Default|SetTargets _outactors)
  ;[1 1 1] Agarra todas las DROGAS
  (bind _outactors_2 (Actor|GetAllActorsOfClass "/Game/Blueprints/Pills.Pills_C"))
  (Variables|Default|Setpills _outactors_2)
  (CallFunction|WinCondition 0.0))

(fn ConstructionScript)

(fn MAKEALLSPOOKY
  (for _array_element (Variables|Default|GetTargets)
    (Default|ChangetoSpooky _array_element 1 (Variables|/Game/Blueprints/Target.Target_C|GetML _array_element))))
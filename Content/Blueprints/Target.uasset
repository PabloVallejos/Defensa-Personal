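; Target actor that is destroyed on taking any damage and can trigger a "Spooky" mode on the first-person character.
; When its Spooky flag is set, overlap begin and end with an actor tagged Player call ActivateTest and DeactivateTest on BP_FirstPersonCharacter.
; The character is fetched through GetActorOfClass rather than taken from the overlapping actor.
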(event Collision|EventActorBeginOverlap
  (params (OtherActor :type Actor%20Object%20Reference))
  ;[1 1 1] Manejo del modo Spooky
  ;;[1 1 1] Activa modo Spooky
  (if (Actor|ActorHasTag OtherActor "Player")
    (if (Variables|Default|GetSpooky)
      (bind _returnvalue (Actor|GetActorOfClass "/Game/FirstPerson/Blueprints/BP_FirstPersonCharacter.BP_FirstPersonCharacter_C"))
      (Default|ActivateTest _returnvalue))))

(event Collision|EventActorEndOverlap
  (params (OtherActor :type Actor%20Object%20Reference))
  ;[1 1 1] Manejo del modo Spooky
  ;;[1 1 1] Desactiva modo Spooky
  (if (Actor|ActorHasTag OtherActor "Player")
    (if (Variables|Default|GetSpooky)
      (bind _returnvalue (Actor|GetActorOfClass "/Game/FirstPerson/Blueprints/BP_FirstPersonCharacter.BP_FirstPersonCharacter_C"))
      (Default|DeactivateTest _returnvalue))))

(event Game|Damage|EventAnyDamage
  (params (Damage :type Float%20%28single-precision%29) (DamageType :type Damage%20Type%20Object%20Reference) (InstigatedBy :type Controller%20Object%20Reference) (DamageCauser :type Actor%20Object%20Reference))
  ;[1 1 1] Destruye el objeto cuando recibe daño
  (Actor|DestroyActor))

(fn ConstructionScript)